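; BP_Projectile is a projectile that destroys enemies and health packs it hits, awarding score for enemy kills.
; Tick moves it along world X at its Speed with a swept offset.
; The mesh's hit event casts the other actor to BP_HealthPack or BP_Enemy, destroying both it and the projectile on a match.
; Only enemy hits update the Player's score, and other hits leave the projectile alive.
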(event OnComponentHit(StaticMeshComponent)
  (params (HitComponent :type Primitive%20Component%20Object%20Reference) (OtherActor :type Actor%20Object%20Reference) (OtherComp :type Primitive%20Component%20Object%20Reference) (NormalImpulse :type Vector :default "0, 0, 0") (Hit :type Hit%20Result%20Structure%20%28by%20ref%29))
  (bind _asbp_health_pack (Utilities|Casting|CastToBP_HealthPack OtherActor)
    (:then
      (Actor|DestroyActor _asbp_health_pack)
      (Actor|DestroyActor))
    (:CastFailed
      (bind _asbp_enemy (Utilities|Casting|CastToBP_Enemy OtherActor))
      (Actor|DestroyActor _asbp_enemy)
      (Actor|DestroyActor)
      (Default|UpdateScore (Variables|Default|GetPlayer) 5))))

(event EventBeginPlay)

(event Collision|EventActorBeginOverlap
  (params (OtherActor :type Actor%20Object%20Reference)))

(event EventTick
  (params (DeltaSeconds :type Float%20%28single-precision%29))
  (Transformation|AddActorWorldOffset (Math|Vector|MakeVector (* DeltaSeconds (Variables|Default|GetSpeed)) 0.0 0.0) true))

(fn ConstructionScript)